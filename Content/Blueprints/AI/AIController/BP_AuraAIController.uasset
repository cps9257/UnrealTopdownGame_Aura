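; BP_AuraAIController is an AI controller that turns perception events into Blackboard data.
; On each target perception update it stores the actor and stimulus, then branches on the stimulus's sense class.
; Sight and damage write the actor to TargetToFollow, while hearing writes the stimulus location to TargetLocation.
; It never checks whether the stimulus was successfully sensed, so losing sight also sets TargetToFollow.
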(event OnTargetPerceptionUpdated(AIPerception)
  (params (Actor :type Actor%20Object%20Reference) (Stimulus :type AI%20Stimulus%20Structure))
  (Variables|Default|SetDetectedTarget Actor)
  (bind _output_get (Variables|Default|SetStimulus Stimulus))
  (bind _returnvalue (Class|AIPerceptionSystem|GetSenseClassforStimulus _output_get))
  (Variables|Default|SetSense _returnvalue)
  (if (== (Variables|Default|GetSense) "/Script/AIModule.AISense_Sight")
    (AI|Components|Blackboard|SetValueasObject (Variables|Default|GetBlackboard) (Utilities|Name|MakeLiteralName "TargetToFollow") (Variables|Default|GetDetectedTarget))
    (elif (== (Variables|Default|GetSense) "/Script/AIModule.AISense_Hearing")
      (AI|Components|Blackboard|SetValueasVector (Variables|Default|GetBlackboard) (Utilities|Name|MakeLiteralName "TargetLocation") (.StimulusLocation (Utilities|Struct|BreakAIStimulus (Variables|Default|GetStimulus))))
      (elif (== (Variables|Default|GetSense) "/Script/AIModule.AISense_Damage")
        (AI|Components|Blackboard|SetValueasObject (Variables|Default|GetBlackboard) (Utilities|Name|MakeLiteralName "TargetToFollow") (Variables|Default|GetDetectedTarget))))))

(event EventBeginPlay)

(event EventTick
  (params (DeltaSeconds :type Float%20%28single-precision%29)))

(fn ConstructionScript)